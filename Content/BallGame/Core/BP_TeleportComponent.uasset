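; BP_TeleportComponent is a scene component that lets its owning actor teleport to an aimed point.
; On BeginPlay it spawns a hidden BP_TeleportTarget marker, which StartTeleport reveals.
; While teleporting, Tick traces forward along the component, projects the hit onto the navigation mesh and moves the marker there.
; StopTeleport ends aiming and, only if the trace hit, moves the owner to that point and hides the marker.
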(event EventBeginPlay
  (Variables|Default|SetTeleportActor (Components|GetOwner))
  (bind _returnvalue (Game|SpawnActorfromClass "/Game/BallGame/BP_TeleportTarget.BP_TeleportTarget_C" (Math|Transform|MakeTransform "0, 0, 0") "Undefined" 0 0))
  (bind _output_get (Variables|Default|SetTeleportTarget _returnvalue))
  (Rendering|SetVisibility (Variables|/Game/BallGame/BP_TeleportTarget.BP_TeleportTarget_C|GetSphere _output_get) false false))

(event EventTick
  (params (DeltaSeconds :type Float%20%28single-precision%29))
  (if (Variables|Default|GetbIsTeleporting)
    (CallFunction|DetectHitPoint)))

(fn StartTeleport
  (Variables|Default|SetbIsTeleporting true)
  (Rendering|SetVisibility (Variables|/Game/BallGame/BP_TeleportTarget.BP_TeleportTarget_C|GetSphere (Variables|Default|GetTeleportTarget)) true false))

(fn StopTeleport
  (Variables|Default|SetbIsTeleporting false)
  (if (Variables|Default|GetbHitDetected)
    (Transformation|SetActorLocation (Variables|Default|GetTeleportActor) (Variables|Default|GetHitPoint) false false)
    (Rendering|SetVisibility (Variables|/Game/BallGame/BP_TeleportTarget.BP_TeleportTarget_C|GetSphere (Variables|Default|GetTeleportTarget)) false false)))

(fn DetectHitPoint
  (bind _returnvalue (Transformation|GetWorldLocation))
  (bind _teleporttarget (Variables|Default|GetTeleportTarget))
  (bind (_outhit _returnvalue_2) (Collision|LineTraceByChannel _returnvalue (+ _returnvalue (* (Math|Vector|GetForwardVector) (Variables|Default|GetDistance))) "TraceTypeQuery1" false 0 "None"))
  (Variables|Default|SetbHitDetected _returnvalue_2)
  (bind _output_get (Variables|Default|SetHitPoint (.ProjectedLocation (AI|Navigation|ProjectPointtoNavigation (.location _outhit) 0 0 "0, 0, 0"))))
  (Utilities|IsValid _teleporttarget
    (:Is%20Valid
      (Transformation|SetActorLocation _teleporttarget _output_get false false))))